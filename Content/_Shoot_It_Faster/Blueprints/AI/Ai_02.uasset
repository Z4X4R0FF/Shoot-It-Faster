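; AI controller that sends its pawn wandering between random TargetPoints and chases the first-person character when spotted.
; BeginPlay gathers every TargetPoint in the level, and Tick picks one at random whenever no target is active.
; Each tick also fires a fan of visibility line traces centred on the pawn's forward vector, retargeting on a character hit.
; Target changes stop movement and start AI MoveTo, whose success or failure clears the target flag.
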(event `self.ReceiveBeginPlay`
  ;[1 0 0] get all patrol points
  (bind _outactors (`GameplayStatics.GetAllActorsOfClass` "/Script/Engine.TargetPoint"))
  (set `self.TargetPoints` _outactors))

(event `self.ReceiveTick`
  (params (DeltaSeconds :type "Float (single-precision)"))
  (bind _returnvalue (`self.K2_GetPawn`))
  (bind _targetpoints (`self.TargetPoints`))
  (bind _returnvalue_2 (`self.K2_GetActorLocation` _returnvalue))
  ;[1 0.6094 0] process ai
  (`|ExecutionSequence`
    (:`then_0`
      ;;[0 1 0.2266] Move to patrol point
      (if (not (`self.HasTarget`))
        (bind _output_get (set `self.currentTarget` (`KismetMathLibrary.RandomIntegerInRange` 0 (- (`KismetArrayLibrary.Array_Length` _targetpoints) 1))))
        (set `self.ActorTarget` (`|GetArrayItem` _targetpoints _output_get))
        (`self.OnTargetChanged`)))
    (:`then_1`
      ;;[0 1 0.1328] Line of sight
      (for _index (range (+ (`self.NumTraces`) 1))
        (bind (_outhit _returnvalue_3) (`KismetSystemLibrary.LineTraceSingle` :`Start` _returnvalue_2 :`End` (+ (* (`KismetMathLibrary.GreaterGreater_VectorRotator` (`KismetMathLibrary.GreaterGreater_VectorRotator` (`self.GetActorForwardVector` _returnvalue) (`KismetMathLibrary.MakeRotator` 0.0 0.0 (/ (* (`self.NumTraces`) (`self.Degrees per trace`)) -2.0))) (`KismetMathLibrary.MakeRotator` 0.0 0.0 (* _index (`self.Degrees per trace`)))) 2000.0) _returnvalue_2) :`TraceChannel` "TraceTypeQuery1" :`DrawTime` 0.0))
        ;;[0.9453 1 0] move to spotted [player
        (if _returnvalue_3
          (bind _asfirst_person_character (cast `/Game/_Shoot_It_Faster/Blueprints/Character_Blueprints/FirstPersonCharacter` (`.HitActor` (`GameplayStatics.BreakHitResult` _outhit))))
          (if (!= (`self.ActorTarget`) _asfirst_person_character)
            (set `self.ActorTarget` _asfirst_person_character)
            (`self.OnTargetChanged`)))))))

(event `OnTargetChanged`
  (bind _returnvalue (`self.K2_GetPawn`))
  ;[1 0 0.07031] Comment
  (`NavMovementComponent.StopActiveMovement` (`Pawn.GetMovementComponent` _returnvalue))
  (`|AIMoveTo` _returnvalue (0.0 0.0 0.0) (`self.ActorTarget`) 0.0
    (:`then`
      (set `self.HasTarget` true))
    (:`OnSuccess`
      (set `self.HasTarget` false :!label _label))
    (:`OnFail`
      (goto _label))))

(fn `UserConstructionScript`)
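; BP_BasicMob is a basic enemy that explodes when the player enters its Explosion overlap, dealing base damage and killing itself.
; On BeginPlay it scales the GameInstance's mob attributes by the selected difficulty's multipliers and writes them to its Combatant.
; A speed dispatcher sets walk and crouch speeds from the move-speed attribute.
; ApplyAttributeDamage routes damage through Combatant, notifying the game mode and destroying the mob at zero or less.
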(event `self.ReceiveBeginPlay`
  (`self.SetMobAttributes`)
  (bind _assifbase_game_mode (cast `/Game/_Shoot_It_Faster/Blueprints/SIFBaseGameMode` (`GameplayStatics.GetGameMode`)))
  (set `self.Gamemode` _assifbase_game_mode)
  (add `self.SpeedParametersDispatcher` (delegate `UpdateCharacterSpeedParameters`))
  (`self.SpeedParametersDispatcher`))

(event `UpdateCharacterSpeedParameters`
  (bind _charactermovement (`self.CharacterMovement`))
  (bind _value (`BlueprintMapLibrary.Map_Find` (`CombatantComponent.GetCurrentAttributeValues` (`self.Combatant`)) "/Game/_Shoot_It_Faster/Common/Character/Attributes/MoveSpeedAttribute.MoveSpeedAttribute"))
  ;[0 1 0.3672] updates character speed parameters
  (set `CharacterMovementComponent.MaxWalkSpeed` _value _charactermovement)
  (set `CharacterMovementComponent.MaxWalkSpeedCrouched` (/ _value 2.0) _charactermovement))

(event `self.Explosion.OnComponentBeginOverlap`
  (params (OverlappedComponent :type "PrimitiveComponent Object Reference") (OtherActor :type "Actor Object Reference") (OtherComp :type "PrimitiveComponent Object Reference") (OtherBodyIndex :type Integer) (bFromSweep :type Boolean) (SweepResult :type "HitResult Structure (by ref)"))
  (bind _returnvalue (`SceneComponent.K2_GetComponentLocation` (`self.Explosion`)))
  (bind _asfirst_person_character (cast `/Game/_Shoot_It_Faster/Blueprints/Character_Blueprints/FirstPersonCharacter` OtherActor))
  (`GameplayStatics.PlaySoundAtLocation` "/Game/StarterContent/Audio/Explosion01.Explosion01" _returnvalue (struct) 1.0 1.0 0.0 null null null)
  (`GameplayStatics.SpawnEmitterAtLocation` "/Game/FXVarietyPack/Particles/P_ky_explosion.P_ky_explosion" _returnvalue)
  (`/Game/_Shoot_It_Faster/Blueprints/Character_Blueprints/FirstPersonCharacter.TakeDamage` _asfirst_person_character "/Game/_Shoot_It_Faster/Common/Character/Attributes/HealthAttribute.HealthAttribute" (`BlueprintMapLibrary.Map_Find` (`self.DefaultCharacterAttributeValues`) "/Game/_Shoot_It_Faster/Common/Character/Attributes/BaseDamageAttribute.BaseDamageAttribute"))
  (`self.ApplyAttributeDamage` "/Game/_Shoot_It_Faster/Common/Character/Attributes/HealthAttribute.HealthAttribute" 10000.0))

(fn `ApplyAttributeDamage`
  (params (`Omega Attribute` :type "OmegaAttribute Object Reference") (Damage :type "Float (double-precision)"))
  (bind _combatant (`self.Combatant`))
  (bind _value (`BlueprintMapLibrary.Map_Find` (`CombatantComponent.GetCurrentAttributeValues` _combatant) `Omega Attribute`))
  (`CombatantComponent.ApplyAttributeDamage` _combatant `Omega Attribute` Damage null null)
  (`KismetSystemLibrary.PrintString` (`KismetStringLibrary.Concat_StrStr` "Damage to mob is " (`KismetStringLibrary.Conv_DoubleToString` Damage) ". Remaining health is " (`KismetStringLibrary.Conv_DoubleToString` _value)))
  (if (<= _value 0.0)
    (`/Game/_Shoot_It_Faster/Blueprints/SIFBaseGameMode.MobDeathDispatcher` (`self.Gamemode`))
    (`self.K2_DestroyActor`)))

(fn `SetMobAttributes`
  (locals (`current attribute` :type "OmegaAttribute Object Reference"))
  (bind _defaultcharacterattributevalues (`self.DefaultCharacterAttributeValues`))
  (bind _asglobal_game_instance (cast `/Game/_Shoot_It_Faster/Common/GameInstance/GlobalGameInstance` (`GameplayStatics.GetGameInstance`)))
  (bind _basicmobparams (`/Game/_Shoot_It_Faster/Common/GameInstance/GlobalGameInstance.BasicMobParams` _asglobal_game_instance))
  (bind _keys (`BlueprintMapLibrary.Map_Keys` _basicmobparams))
  (bind _values (`BlueprintMapLibrary.Map_Values` _basicmobparams))
  (for (_array_element _array_index) _values
    (bind _output (`|GetArrayItem` _keys _array_index))
    (bind (_output_id _output_name _output_attributemultipliers) (break `/Game/_Shoot_It_Faster/Common/Structs/Struct_GameDifficult` (`|GetArrayItem` (`/Game/_Shoot_It_Faster/Common/GameInstance/GlobalGameInstance.Difficulties` _asglobal_game_instance) (`/Game/_Shoot_It_Faster/Common/GameInstance/GlobalGameInstance.SelectedDifficultIndex` _asglobal_game_instance))))
    (`BlueprintMapLibrary.Map_Add` _defaultcharacterattributevalues _output (* _array_element (`BlueprintMapLibrary.Map_Find` _output_attributemultipliers _output))))
  (`CombatantComponent.SetCurrentAttributeValues` (`self.Combatant`) _defaultcharacterattributevalues))

(fn `UserConstructionScript`)
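; Main-menu preview actor that generates a random character with a look and stats.
; GenerateCharacter first applies a randomly picked material with a random Color parameter to the mesh as a dynamic instance.
; It then rolls five Omega attributes (health, move speed, armor, gun damage, reload speed) as 1–10 scores mapped to gameplay ranges.
; Skin and attributes are stored in GeneratedCharParameters and broadcast with the character ID through OnCharGenerationEnded.
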(fn `GenerateCharacter`
  (bind (_generatedcharparameters_skin _generatedcharparameters_attributes) (break `/Game/_Shoot_It_Faster/Common/Structs/Struct_CharacterParams` (`self.generatedCharParameters`)))
  (`self.GenerateCharacterLook`)
  (`|ExecutionSequence`
    (:`then_0`
      (bind (_omega_attribute_out _characterattributevalue) (`self.GetRandomCharacterAttributeValue` 1 10 50.0 250.0 "/Game/_Shoot_It_Faster/Common/Character/Attributes/HealthAttribute.HealthAttribute")))
    (:`then_1`
      (bind (_omega_attribute_out_2 _characterattributevalue_2) (`self.GetRandomCharacterAttributeValue` 1 10 400.0 1200.0 "/Game/_Shoot_It_Faster/Common/Character/Attributes/MoveSpeedAttribute.MoveSpeedAttribute")))
    (:`then_2`
      (bind (_omega_attribute_out_3 _characterattributevalue_3) (`self.GetRandomCharacterAttributeValue` 1 10 0.5 2.0 "/Game/_Shoot_It_Faster/Common/Character/Attributes/ArmorAttribute.ArmorAttribute" 2)))
    (:`then_3`
      (bind (_omega_attribute_out_4 _characterattributevalue_4) (`self.GetRandomCharacterAttributeValue` 1 10 0.5 2.0 "/Game/_Shoot_It_Faster/Common/Character/Attributes/GunDamageMultiplierAttribute.GunDamageMultiplierAttribute" 2)))
    (:`then_4`
      (bind (_omega_attribute_out_5 _characterattributevalue_5) (`self.GetRandomCharacterAttributeValue` 1 10 0.5 2.0 "/Game/_Shoot_It_Faster/Common/Character/Attributes/ReloadSpeedMultiplierAttribute.ReloadSpeedMultiplierAttribute" 2)))
    (:`then_5`
      (`|VariableSetRef` _generatedcharparameters_attributes (`|MakeMap` _omega_attribute_out _characterattributevalue _omega_attribute_out_2 _characterattributevalue_2 _omega_attribute_out_3 _characterattributevalue_3 _omega_attribute_out_4 _characterattributevalue_4 _omega_attribute_out_5 _characterattributevalue_5))
      (`self.OnCharGenerationEnded` (`self.CharacterID`) (`self.generatedCharParameters`)))))

(fn `GenerateCharacterLook`
  (bind _charmaterials (`self.CharMaterials`))
  (bind _generatedcharparameters_skin (break `/Game/_Shoot_It_Faster/Common/Structs/Struct_CharacterParams` (`self.generatedCharParameters`)))
  (bind _returnvalue (`KismetMathLibrary.MakeRandomStream` (`KismetMathLibrary.RandomInteger` 5000000)))
  (bind _returnvalue_2 (`PrimitiveComponent.CreateDynamicMaterialInstance` (`self.CharacterMesh`) 0 (`|GetArrayItem` _charmaterials (`KismetMathLibrary.RandomIntegerFromStream` (`KismetArrayLibrary.Array_Length` _charmaterials) _returnvalue)) "None"))
  (bind _output_get (set `self.Color` (make `LinearColor` (`KismetMathLibrary.RandomFloatInRangeFromStream` 0.0 1.0 _returnvalue) (`KismetMathLibrary.RandomFloatInRangeFromStream` 0.0 1.0 _returnvalue) (`KismetMathLibrary.RandomFloatInRangeFromStream` 0.0 1.0 _returnvalue))))
  (`MaterialInstanceDynamic.SetVectorParameterValue` _returnvalue_2 "Color" _output_get)
  (`|VariableSetRef` _generatedcharparameters_skin _returnvalue_2))

(fn `GetRandomCharacterAttributeValue`
  (params (Min :type Integer) (Max :type Integer) (AttributeMin :type "Float (double-precision)") (AttributeMax :type "Float (double-precision)") (`Omega attribute` :type "OmegaAttribute Object Reference") (`Round Decimals` :type Integer))
  (returns (`Omega Attribute out` :type "OmegaAttribute Object Reference") (CharacterAttributeValue :type "/Game/_Shoot_It_Faster/Common/Structs/Struct_CharacterAttributeValue Structure"))
  (bind _returnvalue (`KismetMathLibrary.RandomIntegerInRangeFromStream` Min Max (`KismetMathLibrary.MakeRandomStream` (`KismetMathLibrary.RandomInteger` 5000000))))
  (return `Omega attribute` (make `/Game/_Shoot_It_Faster/Common/Structs/Struct_CharacterAttributeValue` (`LowEntryExtendedStandardLibrary.RoundDecimals` (`KismetMathLibrary.MapRangeClamped` (`KismetMathLibrary.Conv_IntToDouble` _returnvalue) (`KismetMathLibrary.Conv_IntToDouble` Min) (`KismetMathLibrary.Conv_IntToDouble` Max) AttributeMin AttributeMax) `Round Decimals`) _returnvalue)))

(fn `UserConstructionScript`)
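; BP_Doorway_small is a doorway module with two sliding doors that open automatically when something overlaps its Trigger.
; An overlap counter plays a timeline on each entry and reverses it only when the last overlap ends.
; The timeline lerps both doors apart along local Y from their closed positions by MaxSlide.
; The construction script pre-offsets each door by an open percentage, though the left and right percent variables are applied to opposite doors.
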(event `self.Trigger.OnComponentBeginOverlap`
  (params (OverlappedComponent :type "PrimitiveComponent Object Reference") (OtherActor :type "Actor Object Reference") (OtherComp :type "PrimitiveComponent Object Reference") (OtherBodyIndex :type Integer) (bFromSweep :type Boolean) (SweepResult :type "HitResult Structure (by ref)"))
  (bind (_rightdoorclosed_x _rightdoorclosed_y _rightdoorclosed_z) (`KismetMathLibrary.BreakVector` (`self.RightDoorClosed`)))
  (bind (_leftdoorclosed_x _leftdoorclosed_y _leftdoorclosed_z) (`KismetMathLibrary.BreakVector` (`self.LeftDoorClosed`)))
  (`/Engine/EditorBlueprintResources/StandardMacros.IncrementInt` (`self.OverlapsCount`)
    (:`  `
      (bind (_direction _doorposition) (`Timeline|Timeline_1` :!label _label)
        (:`Update`
          (`SceneComponent.K2_SetRelativeLocation` (`self.door_Left`) (`KismetMathLibrary.MakeVector` _leftdoorclosed_x (`KismetMathLibrary.Lerp` _leftdoorclosed_y (- _leftdoorclosed_y (`self.maxSlide`)) _doorposition) _leftdoorclosed_z) false false)
          (`SceneComponent.K2_SetRelativeLocation` (`self.door_right`) (`KismetMathLibrary.MakeVector` _rightdoorclosed_x (`KismetMathLibrary.Lerp` _rightdoorclosed_y (+ _rightdoorclosed_y (`self.maxSlide`)) _doorposition) _rightdoorclosed_z) false false))))))

(event `self.Trigger.OnComponentEndOverlap`
  (params (OverlappedComponent :type "PrimitiveComponent Object Reference") (OtherActor :type "Actor Object Reference") (OtherComp :type "PrimitiveComponent Object Reference") (OtherBodyIndex :type Integer))
  (bind _overlapscount (`self.OverlapsCount`))
  (`/Engine/EditorBlueprintResources/StandardMacros.DecrementInt` _overlapscount
    (:`  `
      (if (== _overlapscount 0)
        (goto _label :!via `Reverse`)))))

(fn `UserConstructionScript`
  (bind _maxslide (`self.maxSlide`))
  ;[0 0.8828 1] Sets Doors Position at spawn
  (`SceneComponent.K2_AddRelativeLocation` (`self.door_Left`) (`KismetMathLibrary.MakeVector` 0.0 (* (* _maxslide (`self.RightDoor_OpenedPos_percent`)) -1.0)) false false)
  (`SceneComponent.K2_AddRelativeLocation` (`self.door_right`) (`KismetMathLibrary.MakeVector` 0.0 (* _maxslide (`self.LeftDoor_OpenedPos_percent`))) false false))
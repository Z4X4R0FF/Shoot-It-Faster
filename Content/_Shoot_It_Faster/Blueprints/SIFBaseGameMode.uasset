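; Base game mode for a wave-based shooter that runs enemy waves and decides win or loss.
; A self-rearming timer spawns each wave from game instance data at random prison cells, scaling intervals by difficulty and possibly dropping a random power-up at a target point.
; Death dispatchers track living enemies and the player.
; Tick opens the end-game widget on player death, enemy overcrowding, or victory when the final wave is cleared.
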(event `PlayerDead`
  (set `self.isPlayerDead` true))

(event `self.ReceiveBeginPlay`
  ;[0.875 0 1] Begin Play
  (add `self.PlayerDeathDispatcher` (delegate `PlayerDead`))
  (add `self.MobDeathDispatcher` (delegate `mob dead`))
  (bind _asglobal_game_instance (cast `/Game/_Shoot_It_Faster/Common/GameInstance/GlobalGameInstance` (`GameplayStatics.GetGameInstance`)))
  (bind _output_get (set `self.GameInstance` _asglobal_game_instance))
  (bind _outactors (`GameplayStatics.GetAllActorsOfClass` "/Script/Engine.TargetPoint"))
  (set `self.PowerUpSpawns` _outactors)
  (bind _outactors_2 (`GameplayStatics.GetAllActorsOfClass` "/Game/_Shoot_It_Faster/Blueprints/Modules/BP_PrisonCell.BP_PrisonCell_C"))
  (set `self.Spawners` _outactors_2)
  (bind (_selecteddifficult_id _selecteddifficult_name _selecteddifficult_attributemultipliers _selecteddifficult_wavetimelengthmultiplier _selecteddifficult_maxmobscounttolose) (break `/Game/_Shoot_It_Faster/Common/Structs/Struct_GameDifficult` (`/Game/_Shoot_It_Faster/Common/GameInstance/GlobalGameInstance.SelectedDifficult` _output_get)))
  (set `self.MaxAliveEnemies` _selecteddifficult_maxmobscounttolose)
  (`KismetSystemLibrary.K2_SetTimerDelegate` (delegate `StartGame`) 2.0)
  (set `self.TimeUntilNextWave` 2.0))

(event `StartGame`
  ;[0 1 0.8594] Event that will initiate game start
  ;[0.875 0 1] Begin Play
  (`self.StartWave`))

(event `mob dead`
  ;[0.875 0 1] Begin Play
  (`/Engine/EditorBlueprintResources/StandardMacros.DecrementInt` (`self.AliveEnemies`)
    (:`  `
      (`/Engine/EditorBlueprintResources/StandardMacros.IncrementInt` (`self.KillNumber`)))))

(event `StartWave`
  (bind _gameinstance (`self.GameInstance`))
  (bind _currentwave (`self.CurrentWave`))
  (bind _waves (`/Game/_Shoot_It_Faster/Common/GameInstance/GlobalGameInstance.Waves` _gameinstance))
  (bind (_selecteddifficult_id _selecteddifficult_name _selecteddifficult_attributemultipliers _selecteddifficult_wavetimelengthmultiplier) (break `/Game/_Shoot_It_Faster/Common/Structs/Struct_GameDifficult` (`/Game/_Shoot_It_Faster/Common/GameInstance/GlobalGameInstance.SelectedDifficult` _gameinstance)))
  (bind (_output_mobcounts _output_wavemodifiers _output_wavetimelength) (break `/Game/_Shoot_It_Faster/Common/Structs/Struct_Wave` (`|GetArrayItem` _waves _currentwave)))
  (bind _returnvalue (* _output_wavetimelength _selecteddifficult_wavetimelengthmultiplier))
  ;[1 0 0.1172] initializes a new wave
  (`|ExecutionSequence`
    (:`then_0`
      (bind _keys (`BlueprintMapLibrary.Map_Keys` _output_mobcounts))
      (bind _values (`BlueprintMapLibrary.Map_Values` _output_mobcounts))
      (for (_array_element _array_index) _keys
        (`self.SpawnMobs` _array_element (`BlueprintMapLibrary.Map_Find` (`/Game/_Shoot_It_Faster/Common/GameInstance/GlobalGameInstance.MobType-AiController Pairs` _gameinstance) _array_element) (`|GetArrayItem` _values _array_index)))
      (`KismetSystemLibrary.PrintString` (`KismetStringLibrary.Concat_StrStr` "Wave " (`KismetStringLibrary.Conv_IntToString` _currentwave) " Spawned! Wave Length is " (`KismetStringLibrary.Conv_DoubleToString` _returnvalue) " seconds!") false true (struct :`R` 1.0 :`B` 0.683033 :`A` 1.0) 5.0)
      (if (< _currentwave (- (`KismetArrayLibrary.Array_Length` _waves) 1))
        (`/Engine/EditorBlueprintResources/StandardMacros.IncrementInt` (`self.CurrentWave`)
          (:`  `
            (`KismetSystemLibrary.K2_SetTimerDelegate` (delegate `StartWave`) _returnvalue)
            (set `self.TimeUntilNextWave` _returnvalue)))
        (else
          (`KismetSystemLibrary.PrintString` "No more waves!" false true (struct :`R` 1.0 :`B` 0.181484 :`A` 1.0) 10.0)
          (set `self.NoWavesFlag` true))))
    (:`then_1`
      (`self.Try Spawn Power Up`))))

(event `self.ReceiveTick`
  (params (DeltaSeconds :type "Float (single-precision)"))
  (bind _timeuntilnextwave (`self.TimeUntilNextWave`))
  (bind (_selecteddifficult_id _selecteddifficult_name _selecteddifficult_attributemultipliers _selecteddifficult_wavetimelengthmultiplier _selecteddifficult_maxmobscounttolose) (break `/Game/_Shoot_It_Faster/Common/Structs/Struct_GameDifficult` (`/Game/_Shoot_It_Faster/Common/GameInstance/GlobalGameInstance.SelectedDifficult` (`self.GameInstance`))))
  ;[0 0.8359 1] check mob count
  (`|ExecutionSequence`
    (:`then_0`
      (if (>= (`self.AliveEnemies`) _selecteddifficult_maxmobscounttolose)
        (`KismetSystemLibrary.PrintString` "GAME OVER" false true (struct :`R` 1.0 :`B` 0.051084 :`A` 1.0) 10.0)
        (if (not (`self.endgameWidgetSpawned`)) :!label _label
          (bind _returnvalue (`|CreateWidget` "/Game/_Shoot_It_Faster/Widgets/MainMenu/MainMenu_EndGame.MainMenu_EndGame_C"))
          (`UserWidget.AddToPlayerScreen` _returnvalue 0)
          (set `self.endgameWidgetSpawned` true)
          (`/OmegaGameFramework/Blueprints/Macros/OMacros_Player.SetInputModes` (`GameplayStatics.GetPlayerController` 0) false true))))
    (:`then_1`
      (if (>= _timeuntilnextwave 1.0)
        (`KismetSystemLibrary.Delay` 1.0)
        (`/Engine/EditorBlueprintResources/StandardMacros.DecrementFloat` _timeuntilnextwave)))
    (:`then_2`
      (if (`self.NoWavesFlag`)
        (if (== (`self.AliveEnemies`) 0)
          (set `self.isGameOverWIN` true)
          (goto _label))))
    (:`then_3`
      (if (`self.isPlayerDead`)
        (goto _label)))))

(fn `SpawnMobs`
  (params (MobType :type "/Game/_Shoot_It_Faster/Common/E_MobTypes Enum" :default "NewEnumerator0") (MobActor :type "Pawn Class Reference") (Count :type Integer))
  (bind _spawners (`self.Spawners`))
  (for _ (range 1 (+ Count 1))
    (`/Game/_Shoot_It_Faster/Blueprints/Modules/BP_PrisonCell.Spawn Mob` (`|GetArrayItem` _spawners (`KismetMathLibrary.RandomIntegerInRangeFromStream` 0 (- (`KismetArrayLibrary.Array_Length` _spawners) 1) (`KismetMathLibrary.MakeRandomStream` (`KismetMathLibrary.RandomInteger` 1000000)))) MobActor)
    (`/Engine/EditorBlueprintResources/StandardMacros.IncrementInt` (`self.AliveEnemies`))))

(fn `Try Spawn Power Up`
  (bind _powerupspawns (`self.PowerUpSpawns`))
  (bind _returnvalue (`KismetMathLibrary.MakeRandomStream` (`KismetMathLibrary.RandomInteger` 1000000)))
  (bind (_selecteddifficult_id _selecteddifficult_name _selecteddifficult_attributemultipliers _selecteddifficult_wavetimelengthmultiplier _selecteddifficult_maxmobscounttolose _selecteddifficult_powerupspawnchancepercent) (break `/Game/_Shoot_It_Faster/Common/Structs/Struct_GameDifficult` (`/Game/_Shoot_It_Faster/Common/GameInstance/GlobalGameInstance.SelectedDifficult` (`self.GameInstance`))))
  (if (<= (`KismetMathLibrary.RandomIntegerInRangeFromStream` 0 100 _returnvalue) _selecteddifficult_powerupspawnchancepercent)
    (bind _value_ (`|LowEntry_LocalVariable` (`KismetMathLibrary.RandomIntegerInRangeFromStream` 0 3 _returnvalue)))
    (`|SpawnActorFromClass` "/Game/_Shoot_It_Faster/Blueprints/BP_PowerUp.BP_PowerUp_C" (`self.GetTransform` (`|GetArrayItem` _powerupspawns (`KismetMathLibrary.RandomIntegerInRangeFromStream` 0 (- (`KismetArrayLibrary.Array_Length` _powerupspawns) 1) _returnvalue))) "AlwaysSpawn" "OverrideRootScale" null (select `int` _value_ :`0` "/Game/sA_PickupSet_1/Fx/NiagaraSystems/NS_Pickup_3.NS_Pickup_3" :`1` "/Game/sA_PickupSet_1/Fx/NiagaraSystems/NS_Pickup_2.NS_Pickup_2" :`2` "/Game/sA_PickupSet_1/Fx/NiagaraSystems/NS_Pickup_4.NS_Pickup_4" :`3` "/Game/sA_PickupSet_1/Fx/NiagaraSystems/NS_Pickup_5.NS_Pickup_5" :!type "NiagaraSystem Object Reference") (select `int` _value_ :`0` "NewEnumerator0" :`1` "NewEnumerator1" :`2` "NewEnumerator2" :`3` "NewEnumerator3" :!type "/Game/_Shoot_It_Faster/Common/E_PowerUps Enum") null)
    (`KismetSystemLibrary.PrintString` "PowerUP Spawned" true true (struct :`G` 0.66 :`B` 1.0 :`A` 1.0) 10.0)))

(fn `UserConstructionScript`)